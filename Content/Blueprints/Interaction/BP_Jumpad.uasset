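; Jump pad actor that launches a FirstPersonCharacter entering its box trigger toward a Destination offset from the pad.
; On overlap, SuggestProjectileVelocity solves a toss velocity from the character's location, which LaunchCharacter applies with configurable XY/Z overrides.
; The construction script sizes the trigger and runs the same solve from the pad's location, printing whether it succeeds, with optional debug drawing.
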(event `self.Box.OnComponentBeginOverlap`
  (params (OverlappedComponent :type "PrimitiveComponent Object Reference") (OtherActor :type "Actor Object Reference") (OtherComp :type "PrimitiveComponent Object Reference") (OtherBodyIndex :type Integer) (bFromSweep :type Boolean) (SweepResult :type "HitResult Structure (by ref)"))
  (bind _asfirst_person_character (cast `/Game/FirstPersonBP/Blueprints/FirstPersonCharacter` OtherActor))
  (bind _tossvelocity (`GameplayStatics.BlueprintSuggestProjectileVelocity` (`self.K2_GetActorLocation` OtherActor) (+ (`self.K2_GetActorLocation`) (`self.Destination`)) (`self.Launch Speed`) (`self.Override Gravity Z`) "DoNotTrace" 32.0 (`self.Favor High Arc`) (`self.Draw Debug`)))
  (`Character.LaunchCharacter` _asfirst_person_character _tossvelocity (`self.XYOverride`) (`self.ZOverride`)))

(fn `UserConstructionScript`
  (bind _returnvalue (`self.K2_GetActorLocation`))
  (`BoxComponent.SetBoxExtent` (`self.Box`) (`self.TriggerExtent`) true)
  (bind (_tossvelocity _returnvalue_2) (`GameplayStatics.BlueprintSuggestProjectileVelocity` _returnvalue (+ _returnvalue (`self.Destination`)) (`self.Launch Speed`) (`self.Override Gravity Z`) "DoNotTrace" 32.0 (`self.Favor High Arc`) (`self.Draw Debug`)))
  (`KismetSystemLibrary.PrintString` (`KismetStringLibrary.Conv_BoolToString` _returnvalue_2)))