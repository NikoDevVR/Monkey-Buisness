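; BP_Pole_Swing is a swing pole that launches a FirstPersonCharacter forward and upward on contact.
; Two trigger boxes each launch along their own arrow at SwingSpeed plus SwingHeight, overriding existing velocity.
; A RecentlySwung list blocks repeat launches until the character leaves the larger ExitBox.
; The construction script sizes all three boxes from PoleLength.
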(event `self.Box2.OnComponentBeginOverlap`
  (params (OverlappedComponent :type "PrimitiveComponent Object Reference") (OtherActor :type "Actor Object Reference") (OtherComp :type "PrimitiveComponent Object Reference") (OtherBodyIndex :type Integer) (bFromSweep :type Boolean) (SweepResult :type "HitResult Structure (by ref)"))
  (bind _recently_swung (`self.Recently_swung`))
  (bind _asfirst_person_character (cast `/Game/FirstPersonBP/Blueprints/FirstPersonCharacter` OtherActor))
  (if (not (`KismetArrayLibrary.Array_Contains` _recently_swung _asfirst_person_character))
    (`KismetArrayLibrary.Array_Add` _recently_swung _asfirst_person_character)
    (`Character.LaunchCharacter` _asfirst_person_character (+ (* (`SceneComponent.GetForwardVector` (`self.Arrow1`)) (`self.Swing_speed`)) (`KismetMathLibrary.MakeVector` 0.0 0.0 (`self.Swing_Height`))) true true)))

(event `self.Box1.OnComponentBeginOverlap`
  (params (OverlappedComponent :type "PrimitiveComponent Object Reference") (OtherActor :type "Actor Object Reference") (OtherComp :type "PrimitiveComponent Object Reference") (OtherBodyIndex :type Integer) (bFromSweep :type Boolean) (SweepResult :type "HitResult Structure (by ref)"))
  (bind _recently_swung (`self.Recently_swung`))
  (bind _asfirst_person_character (cast `/Game/FirstPersonBP/Blueprints/FirstPersonCharacter` OtherActor))
  (if (not (`KismetArrayLibrary.Array_Contains` _recently_swung _asfirst_person_character))
    (`KismetArrayLibrary.Array_Add` _recently_swung _asfirst_person_character)
    (`Character.LaunchCharacter` _asfirst_person_character (+ (* (`SceneComponent.GetForwardVector` (`self.Arrow`)) (`self.Swing_speed`)) (`KismetMathLibrary.MakeVector` 0.0 0.0 (`self.Swing_Height`))) true true)))

(event `self.Exit Box.OnComponentEndOverlap`
  (params (OverlappedComponent :type "PrimitiveComponent Object Reference") (OtherActor :type "Actor Object Reference") (OtherComp :type "PrimitiveComponent Object Reference") (OtherBodyIndex :type Integer))
  (bind _asfirst_person_character (cast `/Game/FirstPersonBP/Blueprints/FirstPersonCharacter` OtherActor))
  (`KismetArrayLibrary.Array_RemoveItem` (`self.Recently_swung`) _asfirst_person_character))

(fn `UserConstructionScript`
  (`BoxComponent.SetBoxExtent` (`self.Box1`) (`KismetMathLibrary.MakeVector` 30.0 (`self.Pole Length`) 100.0) true)
  (`BoxComponent.SetBoxExtent` (`self.Box2`) (`KismetMathLibrary.MakeVector` 30.0 (`self.Pole Length`) 100.0) true)
  (`BoxComponent.SetBoxExtent` (`self.Exit Box`) (`KismetMathLibrary.MakeVector` 200.0 (+ (`self.Pole Length`) 100.0) 200.0) true))