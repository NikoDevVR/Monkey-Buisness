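; Weapon pickup actor that gives SelectedWeapon to an overlapping FirstPersonCharacter, used either as a respawning pickup or a temporary death drop.
; BeginPlay maps the weapon class to an enum, coloring the light and dynamic material per type and destroying Start Rifle drops.
; Death drops vanish on pickup or timeout; others hide for RespawnTime, then scale back via timeline.
; Tick spins the mesh while another timeline drives height and light intensity.
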(event `self.ReceiveBeginPlay`
  (bind _dynamic_material (`self.Dynamic_material`))
  (bind _dynamic_material_2 (`self.Dynamic_material`))
  (bind _dynamic_material_3 (`self.Dynamic_material`))
  (bind _dynamic_material_4 (`self.Dynamic_material`))
  (bind _dynamic_material_5 (`self.Dynamic_material`))
  (bind _dynamic_material_6 (`self.Dynamic_material`))
  (bind _dynamic_material_7 (`self.Dynamic_material`))
  (`|ExecutionSequence`
    (:`then_0`
      (if (`self.isDeathPickup`)
        (`KismetSystemLibrary.Delay` 10.0)
        (`self.K2_DestroyActor`)))
    (:`then_1`
      (if (`self.Picked up`)
        (`self.start respawn timer`)
        (bind (_direction _newtrack_0 _light) (`Timeline|Timeline_0` :!via `PlayFromStart` :!label _label)
          (:`Update`
            (`SceneComponent.K2_SetRelativeLocation` (`self.StaticMesh`) (`KismetMathLibrary.MakeVector` 0.0 0.0 _newtrack_0) false false)
            (`LightComponent.SetIntensity` (`self.PointLight`) _light)))
        (else
          (goto _label :!via `PlayFromStart`))))
    (:`then_2`
      (bind _returnvalue (`PrimitiveComponent.CreateDynamicMaterialInstance` (`self.StaticMesh`) 0 "/Game/Assets/Materials/Master/M_Master_Flat_Color_No_Noise.M_Master_Flat_Color_No_Noise" "None"))
      (set `self.Dynamic_material` _returnvalue)
      (`|ExecutionSequence`
        (:`then_0`
          (bind _weapon_enum (`/Game/FirstPersonBP/Weapons/Base/Hitscan_BPL.convertWeaponClassToEnum` (`self.Selected_weapon`)))
          (set `self.Weapon` _weapon_enum))
        (:`then_1`
          (switch `/Game/FirstPersonBP/Weapons/Base/Weaponlist` (`self.Weapon`)
            (:`NewEnumerator0`
              (`self.K2_DestroyActor`))
            (:`NewEnumerator1`
              (`StaticMeshComponent.SetStaticMesh` (`self.StaticMesh`) "/Game/Blueprints/Pickups/assets/Models/Weapons/SM_TMP_weapon_pickup.SM_TMP_weapon_pickup")
              (set `self.Selected_weapon` "/Game/FirstPersonBP/Weapons/5_Rifle.5_Rifle_C")
              (`LightComponent.SetLightColor` (`self.PointLight`) (struct :`R` 1.0 :`A` 1.0) true)
              (`MaterialInstanceDynamic.SetVectorParameterValue` _dynamic_material_3 "Color" (struct :`A` 1.0))
              (`MaterialInstanceDynamic.SetScalarParameterValue` _dynamic_material_3 "Roughness" 0.25)
              (`MaterialInstanceDynamic.SetVectorParameterValue` _dynamic_material_3 "Emissive" (struct :`R` 1.0 :`A` 1.0)))
            (:`NewEnumerator2`
              (`StaticMeshComponent.SetStaticMesh` (`self.StaticMesh`) "/Game/Blueprints/Pickups/assets/Models/Weapons/SM_TMP_weapon_pickup.SM_TMP_weapon_pickup")
              (set `self.Selected_weapon` "/Game/FirstPersonBP/Weapons/8_Mining_drill.8_Mining_drill_C")
              (`LightComponent.SetLightColor` (`self.PointLight`) (struct :`G` 0.658824 :`B` 1.0 :`A` 1.0) true)
              (`MaterialInstanceDynamic.SetVectorParameterValue` _dynamic_material_4 "Color" (struct :`A` 1.0))
              (`MaterialInstanceDynamic.SetScalarParameterValue` _dynamic_material_4 "Roughness" 0.25)
              (`MaterialInstanceDynamic.SetVectorParameterValue` _dynamic_material_4 "Emissive" (struct :`G` 0.658824 :`B` 1.0 :`A` 1.0)))
            (:`NewEnumerator3`
              (`StaticMeshComponent.SetStaticMesh` (`self.StaticMesh`) "/Game/Blueprints/Pickups/assets/Models/Weapons/SM_TMP_weapon_pickup.SM_TMP_weapon_pickup")
              (set `self.Selected_weapon` "/Game/FirstPersonBP/Weapons/7_Rocket_Launcher.7_Rocket_Launcher_C")
              (`LightComponent.SetLightColor` (`self.PointLight`) (struct :`R` 1.0 :`G` 0.333333 :`A` 1.0) true)
              (`MaterialInstanceDynamic.SetVectorParameterValue` _dynamic_material_5 "Color" (struct :`A` 1.0))
              (`MaterialInstanceDynamic.SetScalarParameterValue` _dynamic_material_5 "Roughness" 0.25)
              (`MaterialInstanceDynamic.SetVectorParameterValue` _dynamic_material_5 "Emissive" (struct :`R` 1.0 :`G` 0.333333 :`A` 1.0)))
            (:`NewEnumerator4`
              (`StaticMeshComponent.SetStaticMesh` (`self.StaticMesh`) "/Game/Blueprints/Pickups/assets/Models/Weapons/SM_TMP_weapon_pickup.SM_TMP_weapon_pickup")
              (set `self.Selected_weapon` "/Game/FirstPersonBP/Weapons/9_Railgun.9_Railgun_C")
              (`LightComponent.SetLightColor` (`self.PointLight`) (struct :`R` 0.470588 :`B` 1.0 :`A` 1.0) true)
              (`MaterialInstanceDynamic.SetVectorParameterValue` _dynamic_material_6 "Color" (struct :`A` 1.0))
              (`MaterialInstanceDynamic.SetScalarParameterValue` _dynamic_material_6 "Roughness" 0.25)
              (`MaterialInstanceDynamic.SetVectorParameterValue` _dynamic_material_6 "Emissive" (struct :`R` 0.470588 :`B` 1.0 :`A` 1.0)))
            (:`NewEnumerator5`
              (`StaticMeshComponent.SetStaticMesh` (`self.StaticMesh`) "/Game/Blueprints/Pickups/assets/Models/Weapons/SM_TMP_weapon_pickup.SM_TMP_weapon_pickup")
              (set `self.Selected_weapon` "/Game/FirstPersonBP/Weapons/6_Plasma_Generator.6_Plasma_Generator_C")
              (`LightComponent.SetLightColor` (`self.PointLight`) (struct :`G` 1.0 :`B` 0.301961 :`A` 1.0) true)
              (`MaterialInstanceDynamic.SetVectorParameterValue` _dynamic_material_2 "Color" (struct :`A` 1.0))
              (`MaterialInstanceDynamic.SetScalarParameterValue` _dynamic_material_2 "Roughness" 0.25)
              (`MaterialInstanceDynamic.SetVectorParameterValue` _dynamic_material_2 "Emissive" (struct :`G` 1.0 :`B` 0.301961 :`A` 1.0)))
            (:`NewEnumerator6`
              (`StaticMeshComponent.SetStaticMesh` (`self.StaticMesh`) "/Game/Blueprints/Pickups/assets/Models/Weapons/SM_TMP_weapon_pickup.SM_TMP_weapon_pickup")
              (set `self.Selected_weapon` "/Game/FirstPersonBP/Weapons/4_Grenade_Launcher.4_Grenade_Launcher_C")
              (`LightComponent.SetLightColor` (`self.PointLight`) (struct :`R` 0.039216 :`G` 1.0 :`A` 1.0) true)
              (`MaterialInstanceDynamic.SetVectorParameterValue` _dynamic_material_7 "Color" (struct :`A` 1.0))
              (`MaterialInstanceDynamic.SetScalarParameterValue` _dynamic_material_7 "Roughness" 0.25)
              (`MaterialInstanceDynamic.SetVectorParameterValue` _dynamic_material_7 "Emissive" (struct :`R` 0.039216 :`G` 1.0 :`A` 1.0)))
            (:`NewEnumerator7`
              (`StaticMeshComponent.SetStaticMesh` (`self.StaticMesh`) "/Game/Blueprints/Pickups/assets/Models/Weapons/SM_TMP_weapon_pickup.SM_TMP_weapon_pickup")
              (set `self.Selected_weapon` "/Game/FirstPersonBP/Weapons/3_Shotgun.3_Shotgun_C")
              (`LightComponent.SetLightColor` (`self.PointLight`) (struct :`R` 1.0 :`G` 0.203922 :`A` 1.0) true)
              (`MaterialInstanceDynamic.SetVectorParameterValue` _dynamic_material "Color" (struct :`A` 1.0))
              (`MaterialInstanceDynamic.SetScalarParameterValue` _dynamic_material "Roughness" 0.25)
              (`MaterialInstanceDynamic.SetVectorParameterValue` _dynamic_material "Emissive" (struct :`R` 1.0 :`G` 0.203922 :`A` 1.0)))))))))

(event `self.Sphere1.OnComponentBeginOverlap`
  (params (OverlappedComponent :type "PrimitiveComponent Object Reference") (OtherActor :type "Actor Object Reference") (OtherComp :type "PrimitiveComponent Object Reference") (OtherBodyIndex :type Integer) (bFromSweep :type Boolean) (SweepResult :type "HitResult Structure (by ref)"))
  (if (== (`self.GetOwner`) OtherActor)
    _
    (elif (not (`self.Picked up`))
      (`|ExecutionSequence`
        (:`then_0`
          (`|ExecutionSequence`
            (:`then_0`
              (bind (_direction _newtrack_0 _scale) (`Timeline|Respawn` :!via `Stop` :!label _label_2)
                (:`Update`
                  (`LightComponent.SetIntensity` (`self.PointLight`) _newtrack_0)
                  (`SceneComponent.SetRelativeScale3D` (`self.StaticMesh`) (`KismetMathLibrary.Conv_DoubleToVector` _scale)))
                (:`Finished`
                  (`SceneComponent.SetRelativeScale3D` (`self.StaticMesh`) (1.0 1.0 1.0) :!label _label_3)
                  (goto _label :!via `PlayFromStart`))))
            (:`then_1`
              (goto _label_3))))
        (:`then_1`
          (bind _asfirst_person_character (cast `/Game/FirstPersonBP/Blueprints/FirstPersonCharacter` OtherActor))
          (bind _asweapon_base (castclass `/Game/FirstPersonBP/Weapons/Base/Weapon_base` (`self.Selected_weapon`)))
          (`/Game/FirstPersonBP/Blueprints/FirstPersonCharacter.Get weapon` _asfirst_person_character _asweapon_base)
          (if (`self.isDeathPickup`)
            (`self.K2_DestroyActor`)
            (else
              (set `self.Picked up` true :!label _label_4)
              (`SceneComponent.SetRelativeScale3D` (`self.StaticMesh`) (0.0 0.0 0.0))
              (`|ExecutionSequence`
                (:`then_0`
                  (`LightComponent.SetIntensity` (`self.PointLight`) 0.0)
                  (`KismetSystemLibrary.Delay` (`self.respawn time`))
                  (set `self.Picked up` false)
                  (goto _label_2 :!via `PlayFromStart`))
                (:`then_1`
                  (goto _label :!via `Stop`))))))))))

(event `start respawn timer`
  (goto _label_4))

(event `self.ReceiveTick`
  (params (DeltaSeconds :type "Float (single-precision)"))
  (`SceneComponent.K2_AddRelativeRotation` (`self.StaticMesh`) (`KismetMathLibrary.MakeRotator` 0.0 0.0 (* DeltaSeconds 180.0)) false false))

(fn `UserConstructionScript`)