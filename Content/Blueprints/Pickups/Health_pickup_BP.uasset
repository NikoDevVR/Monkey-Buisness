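; Pickup that restores health or armor to the FirstPersonCharacter on overlap, then hides and respawns after a delay.
; The construction script uses Level and IsArmor to set mesh, light, amount, overheal and, unless overridden, respawn time.
; Overlap skips full characters unless overheal is allowed, and Heavy pickups by default begin on their respawn timer.
; Timelines drive the bob, light pulse and respawn scale-in, while Tick spins the mesh.
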(event `self.ReceiveBeginPlay`
  (if (`self.Picked up`)
    (`self.start respawn timer`)
    (bind (_direction _newtrack_0 _light) (`Timeline|Timeline_0` :!via `Stop` :!label _label)
      (:`Update`
        (`SceneComponent.K2_SetRelativeLocation` (`self.StaticMesh`) (`KismetMathLibrary.MakeVector` 0.0 0.0 (select `/Game/Blueprints/Pickups/assets/Health_Armor_Types` (`self.Level`) :`NewEnumerator0` (- _newtrack_0 20.0) :`NewEnumerator1` _newtrack_0 :`NewEnumerator2` (+ _newtrack_0 30.0))) false false)
        (`LightComponent.SetIntensity` (`self.PointLight`) _light)))
    (else
      (goto _label :!via `PlayFromStart`))))

(event `self.Sphere.OnComponentBeginOverlap`
  (params (OverlappedComponent :type "PrimitiveComponent Object Reference") (OtherActor :type "Actor Object Reference") (OtherComp :type "PrimitiveComponent Object Reference") (OtherBodyIndex :type Integer) (bFromSweep :type Boolean) (SweepResult :type "HitResult Structure (by ref)"))
  (bind _health (`self.Health`))
  (bind _can_overheal (`self.Can_overheal`))
  (if (`self.IsArmor`)
    (bind _asfirst_person_character (cast `/Game/FirstPersonBP/Blueprints/FirstPersonCharacter` OtherActor))
    (if (or (not (>= (`/Game/FirstPersonBP/Blueprints/FirstPersonCharacter.Armor` _asfirst_person_character) 100.0)) (`self.Can_overheal`))
      (if (`self.Picked up`) :!label _label_2
        (set `self.Picked up` true :!label _label_3)
        (`SceneComponent.SetRelativeScale3D` (`self.StaticMesh`) (0.0 0.0 0.0))
        (`|ExecutionSequence`
          (:`then_0`
            (`LightComponent.SetIntensity` (`self.PointLight`) 0.0)
            (`KismetSystemLibrary.Delay` (`self.respawn time`))
            (set `self.Picked up` false)
            (bind (_direction _newtrack_0 _scale) (`Timeline|Respawn` :!via `PlayFromStart` :!label _label_4)
              (:`Update`
                (`LightComponent.SetIntensity` (`self.PointLight`) _newtrack_0)
                (`SceneComponent.SetRelativeScale3D` (`self.StaticMesh`) (`KismetMathLibrary.Conv_DoubleToVector` _scale)))
              (:`Finished`
                (`SceneComponent.SetRelativeScale3D` (`self.StaticMesh`) (1.0 1.0 1.0) :!label _label_5)
                (goto _label :!via `PlayFromStart`))))
          (:`then_1`
            (goto _label :!via `Stop`)))
        (else
          (`|ExecutionSequence`
            (:`then_0`
              (`|ExecutionSequence`
                (:`then_0`
                  (goto _label_4 :!via `Stop`))
                (:`then_1`
                  (goto _label_5))))
            (:`then_1`
              (bind _asfirst_person_character_2 (cast `/Game/FirstPersonBP/Blueprints/FirstPersonCharacter` OtherActor))
              (if (`self.IsArmor`)
                (`/Game/FirstPersonBP/Blueprints/FirstPersonCharacter.Heal_Armor` _asfirst_person_character_2 _health _can_overheal)
                (goto _label_3)
                (else
                  (`/Game/FirstPersonBP/Blueprints/FirstPersonCharacter.Heal` _asfirst_person_character_2 _health _can_overheal)
                  (goto _label_3))))))))
    (else
      (bind _asfirst_person_character_3 (cast `/Game/FirstPersonBP/Blueprints/FirstPersonCharacter` OtherActor))
      (if (or (not (>= (`/Game/FirstPersonBP/Blueprints/FirstPersonCharacter.Health` _asfirst_person_character_3) 100.0)) (`self.Can_overheal`))
        (goto _label_2)))))

(event `start respawn timer`
  (goto _label_3))

(event `self.ReceiveTick`
  (params (DeltaSeconds :type "Float (single-precision)"))
  (`SceneComponent.K2_AddRelativeRotation` (`self.StaticMesh`) (`KismetMathLibrary.MakeRotator` 0.0 0.0 (* DeltaSeconds 180.0)) false false))

(fn `UserConstructionScript`
  (bind _cube (`self.Cube`))
  (bind _staticmesh (`self.StaticMesh`))
  (bind _staticmesh_2 (`self.StaticMesh`))
  (bind _pointlight (`self.PointLight`))
  (bind _pointlight_2 (`self.PointLight`))
  (bind _cube_2 (`self.Cube`))
  (`|ExecutionSequence`
    (:`then_0`
      (if (`self.IsArmor`)
        (switch `/Game/Blueprints/Pickups/assets/Health_Armor_Types` (`self.Level`)
          (:`NewEnumerator0`
            (`StaticMeshComponent.SetStaticMesh` _staticmesh "/Game/StarterContent/Props/SM_Lamp_Wall.SM_Lamp_Wall")
            (`LightComponent.SetIntensity` _pointlight_2 1250.0)
            (`LocalLightComponent.SetAttenuationRadius` _pointlight_2 250.0)
            (`SceneComponent.SetVisibility` _cube_2 false false)
            (set `self.Health` 5))
          (:`NewEnumerator1`
            (`StaticMeshComponent.SetStaticMesh` _staticmesh "/Game/Blueprints/Pickups/assets/Models/Armor/SM_Armor_Medium.SM_Armor_Medium")
            (`LightComponent.SetIntensity` _pointlight_2 2500.0)
            (`SceneComponent.SetVisibility` _cube_2 false false)
            (set `self.Health` 25))
          (:`NewEnumerator2`
            (`StaticMeshComponent.SetStaticMesh` (`self.StaticMesh`) "/Game/Blueprints/Pickups/assets/Models/Armor/SM_armor_heavy.SM_armor_heavy")
            (`LightComponent.SetIntensity` _pointlight_2 5000.0)
            (`SceneComponent.SetVisibility` _cube_2 true false)
            (set `self.Health` 100)))
        (`LightComponent.SetLightColor` _pointlight_2 (struct :`R` 0.510417 :`G` 0.414288 :`A` 1.0) true)
        (bind _returnvalue (`PrimitiveComponent.CreateDynamicMaterialInstance` (`self.Cube`) 1 "/Game/Blueprints/Pickups/assets/Models/M_pickup_glow.M_pickup_glow" "None"))
        (`MaterialInstanceDynamic.SetVectorParameterValue` _returnvalue "Color" (struct :`R` 4.0 :`G` 2.409906 :`A` 1.0))
        (else
          (switch `/Game/Blueprints/Pickups/assets/Health_Armor_Types` (`self.Level`)
            (:`NewEnumerator0`
              (`StaticMeshComponent.SetStaticMesh` _staticmesh_2 "/Game/Blueprints/Pickups/assets/Models/Health/SM_Health_Small.SM_Health_Small")
              (`LightComponent.SetIntensity` _pointlight 625.0)
              (`LocalLightComponent.SetAttenuationRadius` _pointlight 250.0)
              (`SceneComponent.SetVisibility` _cube false false)
              (set `self.Health` 5))
            (:`NewEnumerator1`
              (`StaticMeshComponent.SetStaticMesh` _staticmesh_2 "/Game/Blueprints/Pickups/assets/Models/Health/SM_Health_Medium.SM_Health_Medium")
              (`LightComponent.SetIntensity` _pointlight 2500.0)
              (`SceneComponent.SetVisibility` _cube false false)
              (set `self.Health` 25))
            (:`NewEnumerator2`
              (`StaticMeshComponent.SetStaticMesh` (`self.StaticMesh`) "/Game/Blueprints/Pickups/assets/Models/Health/SM_Health_heavy.SM_Health_heavy")
              (`LightComponent.SetIntensity` _pointlight 5000.0)
              (`SceneComponent.SetVisibility` _cube true false)
              (set `self.Health` 100)))
          (`LightComponent.SetLightColor` _pointlight (struct :`G` 0.656275 :`B` 1.0 :`A` 1.0) true))))
    (:`then_1`
      (if (not (`self.Overwrite_respawn_time`))
        (switch `/Game/Blueprints/Pickups/assets/Health_Armor_Types` (`self.Level`)
          (:`NewEnumerator0`
            (set `self.respawn time` 7.5)
            (set `self.Can_overheal` true))
          (:`NewEnumerator1`
            (set `self.respawn time` 15.0))
          (:`NewEnumerator2`
            (set `self.respawn time` 30.0)
            (set `self.Picked up` true)
            (set `self.Can_overheal` true)))))))