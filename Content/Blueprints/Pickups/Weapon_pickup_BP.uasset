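; Weapon pickup that gives a FirstPersonCharacter the selected weapon on sphere overlap, then respawns after RespawnTime.
; The construction script maps the Weapon choice to mesh, granted weapon and light color, warning if Start Rifle is chosen.
; Tick spins the mesh while a timeline drives its height and light intensity.
; Pickup hides the mesh by zero scale and kills the light; a Respawn timeline restores both after the delay.
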(event `self.ReceiveBeginPlay`
  (if (`self.Picked up`)
    (`self.start respawn timer`)
    (bind (_direction _newtrack_0 _light) (`Timeline|Timeline_0` :!via `PlayFromStart` :!label _label)
      (:`Update`
        (`SceneComponent.K2_SetRelativeLocation` (`self.StaticMesh`) (`KismetMathLibrary.MakeVector` 0.0 0.0 _newtrack_0) false false)
        (`LightComponent.SetIntensity` (`self.PointLight`) _light)))
    (else
      (goto _label :!via `PlayFromStart`))))

(event `start respawn timer`
  (set `self.Picked up` true :!label _label_2)
  (`SceneComponent.SetRelativeScale3D` (`self.StaticMesh`) (0.0 0.0 0.0))
  (`|ExecutionSequence`
    (:`then_0`
      (`LightComponent.SetIntensity` (`self.PointLight`) 0.0)
      (`KismetSystemLibrary.Delay` (`self.respawn time`))
      (set `self.Picked up` false)
      (bind (_direction _newtrack_0 _scale) (`Timeline|Respawn` :!via `PlayFromStart`)
        (:`Update`
          (`LightComponent.SetIntensity` (`self.PointLight`) _newtrack_0)
          (`SceneComponent.SetRelativeScale3D` (`self.StaticMesh`) (`KismetMathLibrary.Conv_DoubleToVector` _scale)))
        (:`Finished`
          (`SceneComponent.SetRelativeScale3D` (`self.StaticMesh`) (1.0 1.0 1.0))
          (goto _label :!via `PlayFromStart`))))
    (:`then_1`
      (goto _label :!via `Stop`))))

(event `self.Sphere.OnComponentBeginOverlap`
  (params (OverlappedComponent :type "PrimitiveComponent Object Reference") (OtherActor :type "Actor Object Reference") (OtherComp :type "PrimitiveComponent Object Reference") (OtherBodyIndex :type Integer) (bFromSweep :type Boolean) (SweepResult :type "HitResult Structure (by ref)"))
  (if (not (`self.Picked up`))
    (bind _asfirst_person_character (cast `/Game/FirstPersonBP/Blueprints/FirstPersonCharacter` OtherActor))
    (`/Game/FirstPersonBP/Blueprints/FirstPersonCharacter.Get weapon` _asfirst_person_character (`self.Selected_weapon`))
    (goto _label_2)))

(event `self.ReceiveTick`
  (params (DeltaSeconds :type "Float (single-precision)"))
  (`SceneComponent.K2_AddRelativeRotation` (`self.StaticMesh`) (`KismetMathLibrary.MakeRotator` 0.0 0.0 (* DeltaSeconds 180.0)) false false))

(fn `UserConstructionScript`
  (bind _staticmesh (`self.StaticMesh`))
  (switch `/Game/FirstPersonBP/Weapons/Base/Weaponlist` (`self.Weapon`)
    (:`NewEnumerator0`
      (`KismetSystemLibrary.PrintString` "WARNING: START RIFLE SHOULD NOT BE A PICKUP")
      (`StaticMeshComponent.SetStaticMesh` _staticmesh null)
      (set `self.Selected_weapon` "/Game/FirstPersonBP/Weapons/1_Start_rifle.1_Start_rifle_C")
      (`LightComponent.SetLightColor` (`self.PointLight`) (struct :`R` 1.0 :`G` 0.2903 :`A` 1.0) true))
    (:`NewEnumerator1`
      (`StaticMeshComponent.SetStaticMesh` _staticmesh "/Game/StarterContent/Props/SM_Chair.SM_Chair")
      (set `self.Selected_weapon` "/Game/FirstPersonBP/Weapons/5_Rifle.5_Rifle_C")
      (`LightComponent.SetLightColor` (`self.PointLight`) (struct :`R` 1.0 :`A` 1.0) true))
    (:`NewEnumerator2`
      (`StaticMeshComponent.SetStaticMesh` (`self.StaticMesh`) "/Game/StarterContent/Props/SM_CornerFrame.SM_CornerFrame")
      (set `self.Selected_weapon` "/Game/FirstPersonBP/Weapons/8_Mining_drill.8_Mining_drill_C")
      (`LightComponent.SetLightColor` (`self.PointLight`) (struct :`G` 0.656275 :`B` 1.0 :`A` 1.0) true))
    (:`NewEnumerator3`
      (`StaticMeshComponent.SetStaticMesh` (`self.StaticMesh`) "/Game/Geometry/Meshes/1M_Cube.1M_Cube")
      (set `self.Selected_weapon` "/Game/FirstPersonBP/Weapons/7_Rocket_Launcher.7_Rocket_Launcher_C")
      (`LightComponent.SetLightColor` (`self.PointLight`) (struct :`R` 1.0 :`G` 0.335755 :`A` 1.0) true))))